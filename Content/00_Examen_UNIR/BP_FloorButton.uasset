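; BP_FloorButton is an interactable button that the player toggles with E, switching its status light between on and off materials.
; Box overlaps with BP_ThirdPersonCharacter set PlayerIsInside and swap the button between hover and metal materials.
; Both overlap begin and end call EnableInput, so PlayerIsInside alone gates the key press once input is enabled.
; ButtonActivated holds the toggle state and drives only the light material.
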(event `self.ReceiveBeginPlay`
  (`PrimitiveComponent.SetMaterial` (`self.Status_light`) 0 "/Game/00_Examen_UNIR/M_Emission_btn_off.M_Emission_btn_off"))

(event `self.Box.OnComponentBeginOverlap`
  (params (OverlappedComponent :type "PrimitiveComponent Object Reference") (OtherActor :type "Actor Object Reference") (OtherComp :type "PrimitiveComponent Object Reference") (OtherBodyIndex :type Integer) (bFromSweep :type Boolean) (SweepResult :type "HitResult Structure (by ref)"))
  (cast `/Game/ThirdPerson/Blueprints/BP_ThirdPersonCharacter` OtherActor)
  (set `self.PlayerIsInside` true)
  (`self.EnableInput` (`GameplayStatics.GetPlayerController` 0))
  (`PrimitiveComponent.SetMaterial` (`self.Button`) 0 "/Game/00_Examen_UNIR/M_Emission_btn_hover.M_Emission_btn_hover"))

(event `self.Box.OnComponentEndOverlap`
  (params (OverlappedComponent :type "PrimitiveComponent Object Reference") (OtherActor :type "Actor Object Reference") (OtherComp :type "PrimitiveComponent Object Reference") (OtherBodyIndex :type Integer))
  (cast `/Game/ThirdPerson/Blueprints/BP_ThirdPersonCharacter` OtherActor)
  (set `self.PlayerIsInside` false)
  (`self.EnableInput` (`GameplayStatics.GetPlayerController` 0))
  (`PrimitiveComponent.SetMaterial` (`self.Button`) 0 "/Game/LowPolyAssets/Materials/M_Metal.M_Metal"))

(event `Key|E`
  (params (Key :type "Key Structure"))
  (:`Pressed`
    (if (`self.PlayerIsInside`)
      (bind _output_get (set `self.ButtonActivated` (not (`self.ButtonActivated`))))
      (if _output_get
        (`PrimitiveComponent.SetMaterial` (`self.Status_light`) 0 "/Game/00_Examen_UNIR/M_Emission_btn_on.M_Emission_btn_on")
        (else
          (`PrimitiveComponent.SetMaterial` (`self.Status_light`) 0 "/Game/00_Examen_UNIR/M_Emission_btn_off.M_Emission_btn_off"))))))

(fn `UserConstructionScript`)