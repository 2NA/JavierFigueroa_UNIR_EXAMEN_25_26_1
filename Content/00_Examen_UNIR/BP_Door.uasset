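; BP_Door is a sliding double door actor that other code opens and closes through OpenDoor and CloseDoor events.
; BeginPlay caches each panel's relative location as its closed position.
; A single Timeline drives a vector lerp that slides the panels apart along local X, playing forward to open and reversing to close.
; The Open flag gates each direction: true for opening, false for closing.
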(event `self.ReceiveBeginPlay`
  (set `self.InitPos_RightDoor` (`SceneComponent.RelativeLocation` (`self.Right_Door`)))
  (set `self.InitPos_LeftDoor` (`SceneComponent.RelativeLocation` (`self.Left_Door`))))

(event `AnimationOpenDoor`
  (params (Open :type Boolean))
  (if Open
    (bind (_direction _newtrack_0) (`Timeline|Timeline` :!label _label)
      (:`Update`
        (`SceneComponent.K2_SetRelativeLocation` (`self.Right_Door`) (`KismetMathLibrary.VLerp` (`self.InitPos_RightDoor`) (+ (`self.InitPos_RightDoor`) (110.0 0.0 0.0)) _newtrack_0) false false)
        (`SceneComponent.K2_SetRelativeLocation` (`self.Left_Door`) (`KismetMathLibrary.VLerp` (`self.InitPos_LeftDoor`) (+ (`self.InitPos_LeftDoor`) (-110.0 0.0 0.0)) _newtrack_0) false false)))))

(event `AnimationCloseDoor`
  (params (Open :type Boolean))
  (if (not Open)
    (goto _label :!via `Reverse`)))

(event `/Game/00_Examen_UNIR/BPI_OpenDoor.OpenDoor`
  (params (Open :type Boolean))
  (`self.AnimationOpenDoor` Open))

(event `/Game/00_Examen_UNIR/BPI_OpenDoor.CloseDoor`
  (params (Open :type Boolean))
  (`self.AnimationCloseDoor` Open))

(fn `UserConstructionScript`)